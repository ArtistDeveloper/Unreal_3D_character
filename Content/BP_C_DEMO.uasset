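; BP_C_DEMO is a demo player character with mouse look, movement and a simple PEACE/BATTLE state.
; Turn and look axes drive controller yaw and pitch in any state.
; Forward and right axes add movement along control-rotation vectors, but only while CurrentState is PEACE.
; Pressing NormalAttack sets CurrentState to BATTLE, which stops movement input; nothing in this graph returns it to PEACE.
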(event EventBeginPlay)

(event Collision|EventActorBeginOverlap
  (params (OtherActor :type Actor%20Object%20Reference)))

(event Input|ActionEvents|InputActionNormalAttack
  (params (Key :type Key%20Structure))
  ;[1 1 1] Character 상태변환
  (:Pressed
    (Variables|Default|SetCurrentState "NewEnumerator1")))

(event Input|AxisEvents|InputAxisLook_Up
  (params (AxisValue :type Float%20%28single-precision%29))
  ;[1 1 1] 마우스 회전
  (Pawn|Input|AddControllerPitchInput AxisValue))

(event Input|AxisEvents|InputAxisTurn
  (params (AxisValue :type Float%20%28single-precision%29))
  ;[1 1 1] 마우스 회전
  (Pawn|Input|AddControllerYawInput AxisValue))

(event Input|AxisEvents|InputAxisMoveForward
  (params (AxisValue :type Float%20%28single-precision%29))
  ;[1 1 1] Character Movement
  (switch Utilities|FlowControl|Switch|SwitchonBPE_PlayerState (Variables|Default|GetCurrentState)
    (:NewEnumerator0
      (Pawn|Input|AddMovementInput (Math|Vector|GetForwardVector (Pawn|GetControlRotation :!class /Script/Engine.Pawn)) AxisValue false))))

(event Input|AxisEvents|InputAxisMoveRight
  (params (AxisValue :type Float%20%28single-precision%29))
  ;[1 1 1] Character Movement
  (switch Utilities|FlowControl|Switch|SwitchonBPE_PlayerState (Variables|Default|GetCurrentState)
    (:NewEnumerator0
      (Pawn|Input|AddMovementInput (Math|Vector|GetRightVector (Pawn|GetControlRotation :!class /Script/Engine.Pawn)) AxisValue false))))

(fn ConstructionScript)